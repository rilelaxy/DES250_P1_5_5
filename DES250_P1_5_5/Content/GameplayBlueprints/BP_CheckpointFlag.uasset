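; BP_CheckpointFlag is a checkpoint flag actor that can be switched active or inactive and can set the player's respawn point.
; Activate and Deactivate set IsActive and swap the FlagWedge material between orange and gray.
; UpdateRespawn copies the flag's location and rotation into player 0's AC_Health component.
; DeactivateAll is an empty stub with an unconnected GS_DES250 cast, and the event graph has no active logic.
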(fn `Activate`
  (set `self.IsActive` true)
  (`PrimitiveComponent.SetMaterial` (`self.FlagWedge`) 0 "/Game/DoNotChange/PrototypingAssets/Materials/MI_Basic_Orange.MI_Basic_Orange"))

(fn `Deactivate`
  (set `self.IsActive` false)
  (`PrimitiveComponent.SetMaterial` (`self.FlagWedge`) 0 "/Game/DoNotChange/PrototypingAssets/Materials/MI_Basic_Gray.MI_Basic_Gray"))

(fn `DeactivateAll`)

(fn `UpdateRespawn`
  (bind _returnvalue (`self.GetComponentByClass` (`GameplayStatics.GetPlayerPawn` 0) "/Game/ActorComponents/AC_Health.AC_Health_C"))
  (`/Engine/EditorBlueprintResources/StandardMacros.IsValid` _returnvalue
    (:`Is Valid`
      (set `/Game/ActorComponents/AC_Health.RespawnLocation` (`self.K2_GetActorLocation`) _returnvalue)
      (set `/Game/ActorComponents/AC_Health.RespawnRotation` (`self.K2_GetActorRotation`) _returnvalue))))

(fn `UserConstructionScript`)